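; Player character with stamina-driven parkour and a three-weapon loadout of bow, revolver and tomahawk.
; Dashes, jumps and wall runs spend stamina, which regenerates on the ground.
; Capsule hits start wall runs, which lower gravity and are kept alive on a timeline by two side line traces.
; Weapons attach to hand or holster sockets, aim via camera trace, and return loaded ammo to a shared per-type pool when holstered.
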(event `self.ReceiveBeginPlay`
  (bind _weapons (`self.Weapons`))
  (`|ExecutionSequence`
    (:`then_0`
      (`self.ResetStamina` (`self.MaxStamina`)))
    (:`then_1`
      (bind _returnvalue (`|SpawnActorFromClass` "/Game/Blueprints/BP_Bow.BP_Bow_C" (`KismetMathLibrary.MakeTransform` (0.0 0.0 0.0)) "AlwaysSpawn" "OverrideRootScale" null null))
      (bind _weaponstruct (make `/Game/WeaponStruct` _returnvalue))
      (`KismetArrayLibrary.Array_AddUnique` _weapons _weaponstruct)
      (`self.HolsterWeapon` _weaponstruct)
      (bind _returnvalue_2 (`|SpawnActorFromClass` "/Game/Blueprints/BP_Revolver.BP_Revolver_C" (`KismetMathLibrary.MakeTransform` (0.0 0.0 0.0)) "AlwaysSpawn" "OverrideRootScale" null null))
      (bind _weaponstruct_2 (make `/Game/WeaponStruct` _returnvalue_2 "NewEnumerator1"))
      (`KismetArrayLibrary.Array_AddUnique` _weapons _weaponstruct_2)
      (`self.HolsterWeapon` _weaponstruct_2)
      (bind _returnvalue_3 (`|SpawnActorFromClass` "/Game/Blueprints/BP_Tomahawk.BP_Tomahawk_C" (`KismetMathLibrary.MakeTransform` (0.0 0.0 0.0)) "AlwaysSpawn" "OverrideRootScale" null null))
      (bind _weaponstruct_3 (make `/Game/WeaponStruct` _returnvalue_3 "NewEnumerator2"))
      (`KismetArrayLibrary.Array_AddUnique` _weapons _weaponstruct_3)
      (`self.HolsterWeapon` _weaponstruct_3))
    (:`then_2`
      (`self.AddAmmo` 60 "NewEnumerator1")
      (`self.AddAmmo` 30)
      (`self.SetCurrentWeapon` 0)
      (bind _returnvalue_4 (`|CreateWidget` "/Game/HUD_Widget.HUD_Widget_C" (cast `PlayerController` (`self.GetController`) :!pure true)))
      (`UserWidget.AddToViewport` _returnvalue_4 0))))

(event `self.ReceiveTick`
  (params (DeltaSeconds :type "Float (single-precision)"))
  (if (and (`NavMovementComponent.IsMovingOnGround` (`self.CharacterMovement`)) (< (`self.StaminaLeft`) (`self.MaxStamina`)))
    (`self.ResetStamina` (+ (* DeltaSeconds (`self.StaminaRegenPerSecond`)) (`self.StaminaLeft`)))))

(event `/Game/Blueprints/BPI_Damageable.ApplyDamage`
  (params (Damage :type Integer))
  (bind _output_get (set `self.Health` (- (`self.Health`) Damage)))
  (if (<= _output_get 0)
    (`KismetSystemLibrary.PrintString` "DEAD")))

(event `InputAction|Dash`
  (params (Key :type "Key Structure"))
  (:`Pressed`
    (if (`self.CanDash`)
      (`self.ConsumeStamina` 0.5
        (:`Consumed`
          (set `self.CanDash` false)
          (`Timeline|Timeline_0` :!via `PlayFromStart`
            (:`Update`
              (`self.LaunchCharacter` (* 105.0 (+ (* (`self.GetActorRightVector`) (`self.RightAxis`)) (* (`self.ForwardAxis`) (`self.GetActorForwardVector`))))))
            (:`Finished`
              (`KismetSystemLibrary.Delay` 0.1)
              (set `self.CanDash` true))))))))

(event `InputAxis|Turn Right / Left Mouse`
  (params (AxisValue :type "Float (single-precision)"))
  (`self.AddControllerYawInput` AxisValue))

(event `InputAxis|Look Up / Down Mouse`
  (params (AxisValue :type "Float (single-precision)"))
  (`self.AddControllerPitchInput` AxisValue))

(event `InputAxis|Move Forward / Backward`
  (params (AxisValue :type "Float (single-precision)"))
  (bind (_returnvalue_roll _returnvalue_pitch _returnvalue_yaw) (`KismetMathLibrary.BreakRotator` (`self.GetControlRotation`)))
  (bind _output_get (set `self.ForwardAxis` AxisValue))
  (`self.AddMovementInput` (`KismetMathLibrary.GetForwardVector` (`KismetMathLibrary.MakeRotator` 0.0 0.0 _returnvalue_yaw)) _output_get))

(event `InputAxis|Move Right / Left`
  (params (AxisValue :type "Float (single-precision)"))
  (bind (_returnvalue_roll _returnvalue_pitch _returnvalue_yaw) (`KismetMathLibrary.BreakRotator` (`self.GetControlRotation`)))
  (bind _output_get (set `self.RightAxis` (* AxisValue (select `/Game/Enums/EMovementState` "NewEnumerator0" :`NewEnumerator0` 1.0 :`NewEnumerator1` 0.5 :`NewEnumerator2` 1.0))))
  (`self.AddMovementInput` (`KismetMathLibrary.GetRightVector` (`KismetMathLibrary.MakeRotator` _returnvalue_roll 0.0 _returnvalue_yaw)) _output_get))

(event `InputAction|Jump` :overrideparent false
  (params (Key :type "Key Structure"))
  (:`Pressed`
    (`self.OnWall`
      (:`true`
        (`self.ConsumeStamina` 0.5
          (:`Consumed`
            _)))
      (:`false`
        (`self.ConsumeStamina` 1.0
          (:`Consumed`
            _))))
    (`self.LaunchCharacter` (`self.FindLaunchVelocity`) false true)
    (`self.OnWall`
      (:`true`
        (`self.EndWallRun`))))
  (:`Released`
    (`self.StopJumping`)))

(event `ResetStamina`
  (params (Stamina :type "Float (double-precision)"))
  (set `self.StaminaLeft` Stamina))

(event `self.CapsuleComponent.OnComponentHit`
  (params (HitComponent :type "PrimitiveComponent Object Reference") (OtherActor :type "Actor Object Reference") (OtherComp :type "PrimitiveComponent Object Reference") (NormalImpulse :type "Vector Structure") (Hit :type "HitResult Structure (by ref)"))
  (bind (_direction _wallrunside) (`self.FindWallRunDirectionAndSide` Hit_ImpactNormal))
  (`self.OnWall`
    (:`false`
      (if (not (`NavMovementComponent.IsMovingOnGround` (`self.CharacterMovement`)))
        (if (and (>= (`self.StaminaLeft`) (`self.WallrunStaminaPricePerSecond`)) (> (`KismetMathLibrary.VSize2D` (`self.GetHorizontalVelocity`)) 400.0))
          (if (> (`self.StaminaLeft`) 0.0)
            (set `self.WallRunDirection` _direction)
            (set `self.WallRunSide` _wallrunside)
            (if (`self.CanSurfaceBeWallRan` Hit_ImpactNormal)
              (`self.BeginWallRun`))))))))

(event `BeginWallRun`
  (bind _charactermovement (`self.CharacterMovement`))
  (bind (_velocity_x _velocity_y _velocity_z) (`KismetMathLibrary.BreakVector` (`MovementComponent.Velocity` _charactermovement)))
  (set `MovementComponent.Velocity` (`KismetMathLibrary.MakeVector` _velocity_x _velocity_y (/ _velocity_z 2.0)) _charactermovement)
  (set `self.CachedAirControl` (`CharacterMovementComponent.AirControl` _charactermovement))
  (set `self.CachedGravity` (`CharacterMovementComponent.GravityScale` _charactermovement))
  (set `CharacterMovementComponent.AirControl` 1.0 _charactermovement)
  (set `CharacterMovementComponent.GravityScale` 0.15 _charactermovement)
  (set `self.IsWallrunning` true)
  (`Timeline|WallrunTimeline` :!via `PlayFromStart` :!label _label
    (:`Update`
      (`self.UpdateWallRun`))
    (:`Finished`
      (`self.EndWallRun`))))

(event `EndWallRun`
  (bind _charactermovement (`self.CharacterMovement`))
  (set `CharacterMovementComponent.AirControl` (`self.CachedAirControl`) _charactermovement)
  (set `CharacterMovementComponent.GravityScale` (`self.CachedGravity`) _charactermovement)
  (set `self.IsWallrunning` false)
  (goto _label :!via `Stop`))

(event `InputAction|Fire`
  (params (Key :type "Key Structure"))
  (bind _currentweapon_weapon (break `/Game/WeaponStruct` (`self.CurrentWeapon`)))
  (bind _currentweapon_weapon_2 (break `/Game/WeaponStruct` (`self.CurrentWeapon`)))
  (bind _currentweapon_weapon_3 (break `/Game/WeaponStruct` (`self.CurrentWeapon`)))
  (bind _canshoot (`/Game/Blueprints/ABP_Weapon.CanShoot` _currentweapon_weapon))
  (:`Pressed`
    (if _canshoot
      (bind _hitpoint (`self.GetExpectedHitPoint`))
      (`/Game/Blueprints/ABP_Weapon.StartFire` _currentweapon_weapon_2 _hitpoint)))
  (:`Released`
    (if _canshoot
      (bind _hitpoint_2 (`self.GetExpectedHitPoint`))
      (`/Game/Blueprints/ABP_Weapon.EndFire` _currentweapon_weapon_2 _hitpoint_2)
      (if (<= (`/Game/Blueprints/ABP_Weapon.AmmoInWeapon` _currentweapon_weapon_3) 0)
        (`self.TryReloadWeapon`)))))

(event `InputAction|Weapon1`
  (params (Key :type "Key Structure"))
  (:`Pressed`
    (`self.SetCurrentWeapon` 0)))

(event `InputAction|Weapon2`
  (params (Key :type "Key Structure"))
  (:`Pressed`
    (`self.SetCurrentWeapon` 1)))

(event `InputAction|Weapon3`
  (params (Key :type "Key Structure"))
  (:`Pressed`
    (`self.SetCurrentWeapon` 2)))

(event `InputAction|Reload`
  (params (Key :type "Key Structure"))
  (:`Pressed`
    (`self.TryReloadWeapon`)))

(fn `AddAmmo`
  (params (Amount :type Integer) (AmmoType :type "/Game/Enums/EAmmoType Enum" :default "NewEnumerator0"))
  (returns (Added :type Boolean))
  (bind (_currentweapon_weapon _currentweapon_ammotype) (break `/Game/WeaponStruct` (`self.CurrentWeapon`)))
  (bind _value (`BlueprintMapLibrary.Map_Find` (`self.AmmoMap`) (`local.AmmoType`)))
  (bind _value_2 (`BlueprintMapLibrary.Map_Find` (`self.MaxAmmoMap`) (`local.AmmoType`)))
  (bind _returnvalue (select `bool` (and (`KismetSystemLibrary.IsValid` _currentweapon_weapon) (`|EnumEquality` _currentweapon_ammotype (`local.AmmoType`))) :`true` (`/Game/Blueprints/ABP_Weapon.AmmoInWeapon` _currentweapon_weapon)))
  (if (< (+ _value _returnvalue) _value_2)
    (`BlueprintMapLibrary.Map_Add` (`self.AmmoMap`) (`local.AmmoType`) (`KismetMathLibrary.Clamp` (+ Amount _value) 0 (- _value_2 _returnvalue)))
    (return true)
    (else
      (return false))))

(fn `CanSurfaceBeWallRan`
  (params (SurfaceNormal :type "Vector Structure"))
  (returns (NewParam :type Boolean))
  (bind (_x _y _z) (`KismetMathLibrary.BreakVector3f` SurfaceNormal))
  (if (< _z -0.05)
    (return false)
    (elif (< (`KismetMathLibrary.DegAcos` (`KismetMathLibrary.Dot_VectorVector` SurfaceNormal (`KismetMathLibrary.Normal` (`KismetMathLibrary.MakeVector` _x _y)))) (`CharacterMovementComponent.K2_GetWalkableFloorAngle` (`self.CharacterMovement`)))
      (bind _isenough (`self.IsWallrunSurfaceEnough`))
      (return _isenough)
      (else
        (return false)))))

(fn `ClampHorizontalVelocity`
  (bind _returnvalue (/ (`KismetMathLibrary.VSize2D` (`self.GetHorizontalVelocity`)) (`self.SprintingSpeed`)))
  (if (`NavMovementComponent.IsFalling` (`self.CharacterMovement`))
    (if (> _returnvalue 1.0)
      (`self.SetHorizontalVelocity` (`KismetMathLibrary.Conv_VectorToVector2D` (/ (`self.GetHorizontalVelocity`) _returnvalue))))))

(fn `FindLaunchVelocity`
  (returns (LaunchVelocity :type "Vector Structure"))
  (locals (LaunchDirection :type "Vector Structure"))
  (`|ExecutionSequence`
    (:`then_0`
      (if (`self.IsWallrunning`)
        (set `local.LaunchDirection` (`KismetMathLibrary.Cross_VectorVector` (`self.WallRunDirection`) (select `/Game/Enums/EWallRunSide` (`self.WallRunSide`) :`NewEnumerator0` (0.0 0.0 1.0) :`NewEnumerator1` (0.0 0.0 -1.0) :!type "Vector Structure")))
        (elif (`NavMovementComponent.IsFalling` (`self.CharacterMovement`))
          (set `local.LaunchDirection` (+ (* (`self.GetActorRightVector`) (`self.RightAxis`)) (* (`self.ForwardAxis`) (`self.GetActorForwardVector`)))))))
    (:`then_1`
      (return (* (+ (`local.LaunchDirection`) (0.0 0.0 1.0)) (`CharacterMovementComponent.JumpZVelocity` (`self.CharacterMovement`)))))))

(fn `FindWallRunDirectionAndSide`
  (params (`Wall Normal` :type "Vector Structure"))
  (returns (Direction :type "Vector Structure") (WallRunSide :type "/Game/Enums/EWallRunSide Enum"))
  (locals (Side :type "/Game/Enums/EWallRunSide Enum"))
  (bind _output_get (set `local.Side` (select `bool` (> (`KismetMathLibrary.DotProduct2D` (`KismetMathLibrary.Conv_VectorToVector2D` `Wall Normal`) (`KismetMathLibrary.Conv_VectorToVector2D` (`self.GetActorRightVector`))) 0.0) :`false` "NewEnumerator0" :`true` "NewEnumerator1" :!type "/Game/Enums/EWallRunSide Enum")))
  (return (`KismetMathLibrary.Cross_VectorVector` (`local.Wall Normal`) (select `/Game/Enums/EWallRunSide` _output_get :`NewEnumerator0` (0.0 0.0 -1.0) :`NewEnumerator1` (0.0 0.0 1.0) :!type "Vector Structure")) (`local.Side`)))

(fn `GetExpectedHitPoint`
  (returns (HitPoint :type "Vector Structure"))
  (bind _followcamera (`self.FollowCamera`))
  (bind _returnvalue (* (`SceneComponent.GetForwardVector` _followcamera) 100000.0))
  (bind (_outhit _returnvalue_2) (`KismetSystemLibrary.LineTraceSingle` (`SceneComponent.K2_GetComponentLocation` _followcamera) _returnvalue "TraceTypeQuery1"))
  (return (`KismetMathLibrary.SelectVector` (`.Location` (`GameplayStatics.BreakHitResult` _outhit)) _returnvalue _returnvalue_2)))

(fn `GetHorizontalVelocity`
  (returns (ReturnValue :type "Vector2D Structure"))
  (return (`KismetMathLibrary.Conv_VectorToVector2D` (`MovementComponent.Velocity` (`self.CharacterMovement`)))))

(fn `HolsterWeapon`
  (params (Weapon :type "/Game/WeaponStruct Structure"))
  (`self.K2_DetachFromActor` "KeepWorld" "KeepWorld" "KeepWorld")
  (`self.K2_AttachToComponent` (`.Weapon_5_790C56084030CA4A1E0EBEB10794DBEF` (break `/Game/WeaponStruct` Weapon)) (`self.Mesh`) (`/Game/Blueprints/ABP_Weapon.SocketName` (`.Weapon_5_790C56084030CA4A1E0EBEB10794DBEF` (break `/Game/WeaponStruct` Weapon))) "SnapToTarget" "SnapToTarget" "KeepWorld" true)
  (`self.UnloadWeapon` Weapon))

(fn `IsWallrunSurfaceEnough`
  (returns (IsEnough :type Boolean) (HitNormal :type "Vector Structure"))
  (bind (_returnvalue_x _returnvalue_y _returnvalue_z) (`KismetMathLibrary.BreakVector` (`self.K2_GetActorLocation`)))
  (bind _returnvalue (`CapsuleComponent.GetScaledCapsuleRadius` (`self.CapsuleComponent`)))
  (bind _crouchedhalfheight (`CharacterMovementComponent.CrouchedHalfHeight` (`self.CharacterMovement`)))
  (bind _returnvalue_2 (`KismetMathLibrary.MakeVector` _returnvalue_x _returnvalue_y (+ _returnvalue_z _crouchedhalfheight)))
  (bind _returnvalue_3 (`KismetMathLibrary.MakeVector` _returnvalue_x _returnvalue_y (+ _returnvalue_z (* _crouchedhalfheight -1.0))))
  (bind _returnvalue_4 (* (`KismetMathLibrary.Cross_VectorVector` (`self.WallRunDirection`) (select `/Game/Enums/EWallRunSide` (`self.WallRunSide`) :`NewEnumerator0` (0.0 0.0 -1.0) :`NewEnumerator1` (0.0 0.0 1.0) :!type "Vector Structure")) (+ _returnvalue (/ _returnvalue 2.0))))
  (`|ExecutionSequence`
    (:`then_0`
      (bind (_outhit _returnvalue_5) (`KismetSystemLibrary.LineTraceSingle` :`Start` _returnvalue_2 :`End` (+ _returnvalue_2 _returnvalue_4) :`TraceChannel` "TraceTypeQuery1" :`DrawDebugType` "Persistent")))
    (:`then_1`
      (bind (_outhit_2 _returnvalue_6) (`KismetSystemLibrary.LineTraceSingle` :`Start` _returnvalue_3 :`End` (+ _returnvalue_3 _returnvalue_4) :`TraceChannel` "TraceTypeQuery1" :`DrawDebugType` "Persistent" :`TraceColor` (struct :`R` 0.104175 :`B` 1.0 :`A` 1.0))))
    (:`then_2`
      (return (and _returnvalue_5 _returnvalue_6) (`.Normal` (`GameplayStatics.BreakHitResult` _outhit_2))))))

(fn `SetCurrentWeapon`
  (params (WeaponIndex :type Integer))
  (bind _currentweapon_weapon (break `/Game/WeaponStruct` (`self.CurrentWeapon`)))
  (`/Engine/EditorBlueprintResources/StandardMacros.IsValid` _currentweapon_weapon
    (:`Is Valid`
      (if (!= (`KismetArrayLibrary.Array_Find` (`self.Weapons`) (`self.CurrentWeapon`)) WeaponIndex)
        (`self.HolsterWeapon` (`self.CurrentWeapon`))
        (else
          (return))))
    (:`Is Not Valid`
      _))
  (bind _output_get (set `self.CurrentWeapon` (`|GetArrayItem` (`self.Weapons`) WeaponIndex)))
  (`self.K2_AttachToComponent` (break `/Game/WeaponStruct` _output_get) (`self.Mesh`) "right_hand" "SnapToTarget" "SnapToTarget" "KeepWorld" true)
  (`self.TryReloadWeapon`))

(fn `SetHorizontalVelocity`
  (params (NewVelocity :type "Vector2D Structure"))
  (bind _charactermovement (`self.CharacterMovement`))
  (bind (_velocity_x _velocity_y _velocity_z) (`KismetMathLibrary.BreakVector` (`MovementComponent.Velocity` _charactermovement)))
  (set `MovementComponent.Velocity` (`KismetMathLibrary.MakeVector` NewVelocity_X NewVelocity_Y _velocity_z) _charactermovement))

(fn `TryReloadWeapon`
  (locals (AmmoToConsume :type Integer) (CurrentAmmoCount :type Integer))
  (bind (_currentweapon_weapon _currentweapon_ammotype) (break `/Game/WeaponStruct` (`self.CurrentWeapon`)))
  (bind _currentweapon_weapon_2 (break `/Game/WeaponStruct` (`self.CurrentWeapon`)))
  (bind (_currentweapon_weapon_3 _currentweapon_ammotype_2) (break `/Game/WeaponStruct` (`self.CurrentWeapon`)))
  (bind _currentammocount (`local.CurrentAmmoCount`))
  (bind _returnvalue (- (`/Game/Blueprints/ABP_Weapon.MaxAmmo` _currentweapon_weapon_2) (`/Game/Blueprints/ABP_Weapon.AmmoInWeapon` _currentweapon_weapon_2)))
  (bind _output_get (set `local.CurrentAmmoCount` (`BlueprintMapLibrary.Map_Find` (`self.AmmoMap`) _currentweapon_ammotype)))
  (if (> _output_get 0)
    (bind _output_get_2 (set `local.AmmoToConsume` (select `bool` (> _returnvalue _currentammocount) :`false` _returnvalue :`true` _currentammocount)))
    (`/Game/Blueprints/ABP_Weapon.Reload` _currentweapon_weapon_3 _output_get_2)
    (`BlueprintMapLibrary.Map_Add` (`self.AmmoMap`) _currentweapon_ammotype_2 (- (`local.CurrentAmmoCount`) (`local.AmmoToConsume`)))))

(fn `UnloadWeapon`
  (params (Weapon :type "/Game/WeaponStruct Structure"))
  (`BlueprintMapLibrary.Map_Add` (`self.AmmoMap`) Weapon_AmmoType_14_9AC013BE4AD5145906A571B8574F3F26 (+ (`/Game/Blueprints/ABP_Weapon.AmmoInWeapon` Weapon_Weapon_5_790C56084030CA4A1E0EBEB10794DBEF) (`BlueprintMapLibrary.Map_Find` (`self.AmmoMap`) Weapon_AmmoType_14_9AC013BE4AD5145906A571B8574F3F26)))
  (set `/Game/Blueprints/ABP_Weapon.AmmoInWeapon` 0 Weapon_Weapon_5_790C56084030CA4A1E0EBEB10794DBEF)
  (`/Game/Blueprints/ABP_Weapon.ProcessUnload` Weapon_Weapon_5_790C56084030CA4A1E0EBEB10794DBEF))

(fn `UpdateWallRun`
  (bind _charactermovement (`self.CharacterMovement`))
  (bind (_velocity_x _velocity_y _velocity_z) (`KismetMathLibrary.BreakVector` (`MovementComponent.Velocity` _charactermovement)))
  (bind (_velocity_x_2 _velocity_y_2) (`KismetMathLibrary.BreakVector` (`MovementComponent.Velocity` (`self.CharacterMovement`))))
  (if (> (`KismetMathLibrary.VSize2D` (`KismetMathLibrary.MakeVector2D` _velocity_x_2 _velocity_y_2)) 0.1)
    (bind (_isenough _hitnormal) (`self.IsWallrunSurfaceEnough`))
    (if _isenough
      (bind (_direction _wallrunside) (`self.FindWallRunDirectionAndSide` _hitnormal))
      (if (`|EnumEquality` _wallrunside (`self.WallRunSide`))
        (`self.ConsumeStamina` (* (`self.WallrunStaminaPricePerSecond`) (`GameplayStatics.GetWorldDeltaSeconds`))
          (:`Consumed`
            (bind _output_get (set `self.WallRunDirection` _direction))
            (bind (_returnvalue_x _returnvalue_y) (`KismetMathLibrary.BreakVector` (+ (* _output_get 0.2) (`KismetMathLibrary.MakeVector` _velocity_x _velocity_y))))
            (set `MovementComponent.Velocity` (`KismetMathLibrary.MakeVector` _returnvalue_x _returnvalue_y _velocity_z) _charactermovement))
          (:`NotConsumed`
            (`self.EndWallRun` :!label _label)))
        (else
          (goto _label)))
      (else
        (`self.EndWallRun`)))
    (else
      (`self.EndWallRun`))))

(fn `UserConstructionScript`)