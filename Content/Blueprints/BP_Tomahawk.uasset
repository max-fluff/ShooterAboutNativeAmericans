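; BP_Tomahawk is a child weapon Blueprint that fires as a hitscan attack.
; StartFire resolves a hit point from the expected cast point, then applies damage to the hit actor if it implements BPI_Damageable.
; It also spawns the N_Projectile Niagara system at its own location, setting BeamEnd to the hit point.
; StartFire skips the parent implementation, while EndFire (with a zero vector) and Reload defer to it.
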(event `self.ReceiveBeginPlay`)

(fn `EndFire`
  (params (ExpectedCastPoint :type "Vector Structure"))
  (`parent.EndFire` (0.0 0.0 0.0)))

(fn `Reload`
  (params (Amount :type Integer))
  (`parent.Reload` Amount))

(fn `StartFire`
  (params (ExpectedCastPoint :type "Vector Structure"))
  (bind (_hitpoint _hitactor) (`self.GetHitPoint` ExpectedCastPoint))
  (`|ExecutionSequence`
    (:`then_0`
      (bind _asbpi_damageable (cast `/Game/Blueprints/BPI_Damageable` _hitactor))
      (`/Game/Blueprints/BPI_Damageable.ApplyDamage` _asbpi_damageable (`self.Damage`)))
    (:`then_1`
      (if true
        (bind _returnvalue (`NiagaraFunctionLibrary.SpawnSystemAtLocation` "/Game/Effects/N_Projectile.N_Projectile" (`self.K2_GetActorLocation`)))
        (`FXSystemComponent.SetVectorParameter` _returnvalue "BeamEnd" _hitpoint)))))

(fn `UserConstructionScript`)