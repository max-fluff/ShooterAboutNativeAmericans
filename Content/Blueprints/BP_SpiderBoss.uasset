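; Spider boss enemy that bites the nearby player and periodically spawns random batches of regular, skull and dynamite spiders while alive.
; On death it starts a revive timeline, during which a player carrying dynamite can interact to plant it and halt the revival.
; After a short fuse, Blow deals distance-scaled damage to capsule-bearing damageable actors.
; Each blast revives the boss with less health until the third shows the end HUD.
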(event `self.ReceiveTick`
  (params (DeltaSeconds :type "Float (single-precision)"))
  (`parent.ReceiveTick` DeltaSeconds)
  (if (`|EnumInequality` (`self.EnemyState`) "NewEnumerator2")
    (set `self.TimeSinceLastSpawn` (+ (`self.TimeSinceLastSpawn`) DeltaSeconds))
    (if (>= (`self.TimeSinceLastSpawn`) (`self.SpawnDelay`))
      (set `self.TimeSinceLastSpawn` 0.0)
      (`|ExecutionSequence`
        (:`then_0`
          (for _ (range (+ (`KismetMathLibrary.RandomIntegerInRange` 0 4) 1))
            (`|SpawnActorFromClass` "/Game/Blueprints/BP_Spider.BP_Spider_C" (`KismetMathLibrary.MakeTransform` (`SceneComponent.K2_GetComponentLocation` (`self.CapsuleComponent`))) "AdjustIfPossibleButAlwaysSpawn" "OverrideRootScale" null null)))
        (:`then_1`
          (for _ (range (+ (`KismetMathLibrary.RandomIntegerInRange` 0 2) 1))
            (`|SpawnActorFromClass` "/Game/Blueprints/BP_SkullSpider.BP_SkullSpider_C" (`KismetMathLibrary.MakeTransform` (`SceneComponent.K2_GetComponentLocation` (`self.CapsuleComponent`))) "AdjustIfPossibleButAlwaysSpawn" "OverrideRootScale" null null)))
        (:`then_2`
          (for _ (range (+ (`KismetMathLibrary.RandomIntegerInRange` 0 1) 1))
            (`|SpawnActorFromClass` "/Game/Blueprints/BP_DynamiteSpider.BP_DynamiteSpider_C" (`KismetMathLibrary.MakeTransform` (`SceneComponent.K2_GetComponentLocation` (`self.CapsuleComponent`))) "AdjustIfPossibleButAlwaysSpawn" "OverrideRootScale" null null)))))))

(event `self.ReceiveBeginPlay`
  (`parent.ReceiveBeginPlay`)
  (`SceneComponent.SetWorldScale3D` (`self.PaperSprite`) (0.0 0.0 0.0))
  (`SceneComponent.SetWorldScale3D` (`self.Dynamite`) (0.0 0.0 0.0))
  (`AudioComponent.Stop` (`self.Ticking`)))

(event `/Game/Blueprints/BPI_Interactable.Interact`
  (bind _ticking (`self.Ticking`))
  (if (`|EnumEquality` (`self.EnemyState`) "NewEnumerator2")
    (bind _asbp_main_character (cast `/Game/Blueprints/BP_MainCharacter` (`GameplayStatics.GetPlayerCharacter` 0)))
    (if (`/Game/Blueprints/BP_MainCharacter.GotDynamite` _asbp_main_character)
      (set `/Game/Blueprints/BP_MainCharacter.GotDynamite` false _asbp_main_character)
      (`|ExecutionSequence`
        (:`then_0`
          (set `self.Reviving Process` 0.0)
          (bind (_direction _revivingprocess) (`Timeline|ReviveTimeline` :!via `Stop` :!label _label)
            (:`Update`
              (set `self.Reviving Process` _revivingprocess))
            (:`Finished`
              (set `self.Reviving Process` 0.0)
              (if (`|EnumEquality` (`self.EnemyState`) "NewEnumerator2")
                (`self.SetEnemyState` "NewEnumerator0" true)
                (set `self.Health` (* (`self.MaxHealth`) (/ (- 3 (`self.BlownTimes`)) 3)))
                (`SceneComponent.SetWorldScale3D` (`self.PaperSprite`) (0.0 0.0 0.0))))))
        (:`then_1`
          (`SceneComponent.SetWorldScale3D` (`self.PaperSprite`) (0.0 0.0 0.0))
          (`SceneComponent.SetRelativeScale3D` (`self.Dynamite`) (0.3 0.3 0.3))
          (`AudioComponent.Play` _ticking 0.0)
          (`KismetSystemLibrary.Delay` 3.0)
          (`AudioComponent.Stop` _ticking)
          (`self.Blow`))))))

(event `ReviveTimer`
  (goto _label :!via `PlayFromStart`))

(fn `Blow`
  (bind _blowradius (`self.BlowRadius`))
  (`GameplayStatics.SpawnEmitterAtLocation` "/Game/StarterContent/Particles/P_Explosion.P_Explosion" (`SceneComponent.K2_GetComponentLocation` (`self.CapsuleComponent`)) (struct) (7.0 7.0 7.0))
  (`|ExecutionSequence`
    (:`then_0`
      (bind _outactors (`GameplayStatics.GetAllActorsWithInterface` "/Game/Blueprints/BPI_Damageable.BPI_Damageable_C"))
      (for _array_element _outactors
        (bind _returnvalue (`self.GetComponentByClass` _array_element "/Script/Engine.CapsuleComponent"))
        (`/Engine/EditorBlueprintResources/StandardMacros.IsValid` _returnvalue
          (:`Is Valid`
            (bind _asbpi_damageable (cast `/Game/Blueprints/BPI_Damageable` _array_element))
            (bind _returnvalue_2 (`KismetMathLibrary.VSize` (- (`SceneComponent.K2_GetComponentLocation` _returnvalue) (`SceneComponent.K2_GetComponentLocation` (`self.CapsuleComponent`)))))
            (if (< _returnvalue_2 _blowradius)
              (`/Game/Blueprints/BPI_Damageable.ApplyDamage` _asbpi_damageable (`KismetMathLibrary.FTrunc` (* (- 1.0 (/ _returnvalue_2 _blowradius)) (`self.MaxDamage`)))))))))
    (:`then_1`
      (`GameplayStatics.PlaySoundAtLocation` "/Game/Sound/Blow/BigBlow.BigBlow" (`SceneComponent.K2_GetComponentLocation` (`self.CapsuleComponent`)) (struct) 1.0 1.0 0.0 null null null null)
      (`SceneComponent.SetWorldScale3D` (`self.Dynamite`) (0.0 0.0 0.0)))
    (:`then_2`
      (bind _result (`/Engine/EditorBlueprintResources/StandardMacros.IncrementInt` (`self.BlownTimes`))
        (:`  `
          (if (>= _result 3)
            (bind _returnvalue_3 (`GameplayStatics.GetActorOfClass` "/Game/Blueprints/BP_MainCharacter.BP_MainCharacter_C"))
            (`/Game/Blueprints/BP_MainCharacter.ShowEndHud` _returnvalue_3)
            (elif (`|EnumEquality` (`self.EnemyState`) "NewEnumerator2")
              (set `self.Health` (`KismetMathLibrary.FTrunc` (* (/ (`KismetMathLibrary.Conv_IntToDouble` (- 3 (`self.BlownTimes`))) 3.0) (`self.MaxHealth`))))
              (`self.SetEnemyState` "NewEnumerator0" true))))))))

(fn `OnDeath`
  (`GameplayStatics.PlaySoundAtLocation` "/Game/Sound/Insects/Screech.Screech" (`SceneComponent.K2_GetComponentLocation` (`self.CapsuleComponent`)) (struct) 1.0 1.0 0.0 null null null null)
  (set `self.TimeSinceLastSpawn` 0.0)
  (if (<= (`self.BlownTimes`) 2)
    (`SceneComponent.SetRelativeScale3D` (`self.PaperSprite`) (0.015 0.015 0.015))
    (`self.ReviveTimer`)))

(fn `TryAttack`
  (params (DeltaTime :type "Float (double-precision)"))
  (set `self.TimeSinceLastAttack` (+ (`self.TimeSinceLastAttack`) DeltaTime))
  (if (`|EnumEquality` (`self.EnemyState`) "NewEnumerator1")
    (if (< (`KismetMathLibrary.VSize` (- (`SceneComponent.K2_GetComponentLocation` (`self.CapsuleComponent`)) (`SceneComponent.K2_GetComponentLocation` (`Character.Mesh` (`self.Player`))))) 600.0)
      (if (>= (`self.TimeSinceLastAttack`) (`self.AttackDelay`))
        (`/Game/Blueprints/BPI_Damageable.ApplyDamage` (`self.Player`) (`self.DamageAmount`))
        (`GameplayStatics.PlaySound2D` "/Game/Sound/Insects/Bite.Bite" 1.0 1.0 0.0 null null)
        (set `self.TimeSinceLastAttack` 0.0)))))

(fn `UserConstructionScript`
  (`parent.UserConstructionScript`))