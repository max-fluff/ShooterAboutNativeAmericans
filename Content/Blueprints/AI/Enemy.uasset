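; Enemy that shoots the player with a child-actor revolver and rewards them with stamina for damaging it.
; Pawn sensing triggers a timeline that eases clamped pitch and yaw aim values toward the player.
; A line trace confirms the target before a delayed shot, with CanShoot gating fire and a timed reload.
; Damage restores player stamina proportionally, and death plays a sound, disables capsule collision and grants full stamina.
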(event `self.ReceiveBeginPlay`
  (bind _asbp_revolver (cast `/Game/Blueprints/BP_Revolver` (`ChildActorComponent.ChildActor` (`self.Weapon`))))
  (set `self.Revolver` _asbp_revolver))

(event `self.PawnSensing.OnSeePawn`
  (params (Pawn :type "Pawn Object Reference"))
  (if (not (`self.IsDead`))
    (cast `/Game/Blueprints/BP_MainCharacter` Pawn)
    (if (`self.CanShoot`)
      (`self.Aim`)
      (`self.TryShoot`))))

(event `Aim`
  (bind (_returnvalue_roll _returnvalue_pitch _returnvalue_yaw) (`KismetMathLibrary.BreakRotator` (`SceneComponent.K2_GetComponentRotation` (`self.CapsuleComponent`))))
  (bind (_returnvalue_roll_2 _returnvalue_pitch_2 _returnvalue_yaw_2) (`KismetMathLibrary.BreakRotator` (`SceneComponent.K2_GetComponentRotation` (`self.CapsuleComponent`))))
  (bind (_direction _alpha) (`Timeline|Timeline_0` :!via `PlayFromStart`)
    (:`Update`
      (bind (_returnvalue_roll_3 _returnvalue_pitch_3 _returnvalue_yaw_3) (`KismetMathLibrary.BreakRotator` (`KismetMathLibrary.RLerp` (`KismetMathLibrary.MakeRotator` 0.0 (`self.UD`) (+ (`self.LR`) _returnvalue_yaw)) (`KismetMathLibrary.FindLookAtRotation` (`SceneComponent.K2_GetComponentLocation` (`self.Weapon`)) (`self.K2_GetActorLocation` (`GameplayStatics.GetPlayerCharacter` 0))) _alpha)))
      (set `self.UD` (`KismetMathLibrary.FClamp` _returnvalue_pitch_3 -60.0 60.0))
      (set `self.LR` (`KismetMathLibrary.FClamp` (- _returnvalue_yaw_3 _returnvalue_yaw_2) -60.0 60.0)))))

(event `TryShoot`
  (bind _revolver (`self.Revolver`))
  (bind _outhit (`KismetSystemLibrary.LineTraceSingle` (`SceneComponent.K2_GetComponentLocation` (`self.Weapon`)) (`SceneComponent.K2_GetComponentLocation` (`Character.CapsuleComponent` (`GameplayStatics.GetPlayerCharacter` 0))) "TraceTypeQuery2" true))
  (cast `/Game/Blueprints/BP_MainCharacter` (`.HitActor` (`GameplayStatics.BreakHitResult` _outhit)))
  (set `self.CanShoot` false)
  (`KismetSystemLibrary.Delay` 0.5)
  (if (not (`self.IsDead`))
    (`/Game/Blueprints/BP_Revolver.StartShooting` (`self.Revolver`) (`.Location` (`GameplayStatics.BreakHitResult` _outhit)))
    (if (<= (`/Game/Blueprints/ABP_Weapon.AmmoInWeapon` (`self.Revolver`)) 0)
      (`KismetSystemLibrary.Delay` 2.0)
      (set `/Game/Blueprints/ABP_Weapon.AmmoInWeapon` (`/Game/Blueprints/ABP_Weapon.MaxAmmo` _revolver) _revolver))
    (set `self.CanShoot` true)))

(event `/Game/Blueprints/BPI_Damageable.ApplyDamage`
  (params (Damage :type Integer))
  (if (not (`self.IsDead`))
    (bind _output_get (set `self.Health` (- (`self.Health`) Damage)))
    (bind _asbp_main_character (cast `/Game/Blueprints/BP_MainCharacter` (`GameplayStatics.GetPlayerPawn` 0)))
    (`/Game/Blueprints/BP_MainCharacter.Event Restore Stamina` _asbp_main_character (* (/ Damage (`self.MaxHealth`)) (`/Game/Blueprints/BP_MainCharacter.MaxStamina` _asbp_main_character)))
    (if (<= _output_get 0)
      (set `self.IsDead` true)
      (`GameplayStatics.PlaySoundAtLocation` "/Game/Sound/Dying.Dying" (`SceneComponent.K2_GetComponentLocation` (`self.CapsuleComponent`)) (struct) 1.0 1.0 0.0 null null null null)
      (`PrimitiveComponent.SetCollisionEnabled` (`self.CapsuleComponent`) "NoCollision")
      (bind _asbp_main_character_2 (cast `/Game/Blueprints/BP_MainCharacter` (`GameplayStatics.GetPlayerPawn` 0)))
      (`/Game/Blueprints/BP_MainCharacter.Event Restore Stamina` _asbp_main_character_2 (`/Game/Blueprints/BP_MainCharacter.MaxStamina` _asbp_main_character_2)))))

(fn `UserConstructionScript`)