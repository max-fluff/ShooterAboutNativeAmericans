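; Bow weapon that charges while firing is held and launches a BP_Arrow on release.
; Reload spawns an arrow attached to the bow mesh's socket and adds to the ammo count.
; StartFire plays a timeline driving ChargeAmount; EndFire detaches the arrow, fires it toward GetHitPoint's result with that charge, decrements ammo and resets the timeline.
; Unloading destroys the nocked arrow and stops charging, while EndCharge can reverse the charge.
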(event `BeginCharge`
  (`self.Arrow`
    (:`then`
      (bind (_direction _chargeamount) (`Timeline|ChargeTimeline` :!label _label)
        (:`Update`
          (set `self.Charge Amount` _chargeamount))))
    (:`else`)))

(event `EndCharge`
  (`self.Arrow`
    (:`then`
      (goto _label :!via `Reverse`))
    (:`else`)))

(event `StopCharge`
  (`|ExecutionSequence`
    (:`then_0`
      (goto _label :!via `Stop`))
    (:`then_1`
      (goto _label :!via `SetNewTime`))))

(fn `EndFire`
  (params (ExpectedCastPoint :type "Vector Structure"))
  (bind _arrow (`self.Arrow`)
    (:`then`
      (`self.K2_DetachFromActor` _arrow "KeepWorld" "KeepWorld" "KeepWorld")
      (bind _hitpoint (`self.GetHitPoint` ExpectedCastPoint))
      (`/Game/Blueprints/BP_Arrow.Fire` (`self.Arrow`) (`self.Charge Amount`) (`KismetMathLibrary.Normal` (- _hitpoint (`self.K2_GetActorLocation` (`self.Arrow`)))))
      (set `self.Arrow` null)
      (`/Engine/EditorBlueprintResources/StandardMacros.DecrementInt` (`self.AmmoInWeapon`)
        (:`  `
          (`self.StopCharge`))))
    (:`else`)))

(fn `ProcessUnload`
  (bind _arrow (`self.Arrow`)
    (:`then`
      (`self.K2_DestroyActor` _arrow)
      (`self.StopCharge`))
    (:`else`)))

(fn `Reload`
  (params (Amount :type Integer))
  (bind _returnvalue (`|SpawnActorFromClass` "/Game/Blueprints/BP_Arrow.BP_Arrow_C" (`KismetMathLibrary.MakeTransform` (0.0 0.0 0.0)) "Undefined" "OverrideRootScale" null "NewEnumerator2" null))
  (bind _output_get (set `self.Arrow` _returnvalue))
  (`self.K2_AttachToComponent` _output_get (`self.BowMesh`) "arrow_attach_socket" "SnapToTarget" "SnapToTarget" "KeepWorld" true)
  (set `self.AmmoInWeapon` (+ (`self.AmmoInWeapon`) (`local.Amount`)))
  (return))

(fn `StartFire`
  (params (ExpectedCastPoint :type "Vector Structure"))
  (`self.BeginCharge`))

(fn `UserConstructionScript`)