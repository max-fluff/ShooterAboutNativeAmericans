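; Spider boss lair actor that starts the boss encounter once every cobweb column in the level is destroyed.
; On BeginPlay it caches all BP_CobWebColumn actors, then polls them each Tick, recounting destroyed ones and comparing the previous count to the total.
; When all are down, it fires once: removes its cobweb component, moves BP_SpiderBoss to just below the lair's root and plays the aggressive soundtrack.
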(event `self.ReceiveBeginPlay`
  (bind _outactors (`GameplayStatics.GetAllActorsOfClass` "/Game/Blueprints/BP_CobWebColumn.BP_CobWebColumn_C"))
  (set `self.Columns` _outactors))

(event `self.ReceiveTick`
  (params (DeltaSeconds :type "Float (single-precision)"))
  (if (`self.IsDestroyed`)
    _
    (elif (== (`KismetArrayLibrary.Array_Length` (`self.Columns`)) (`self.DestroyedColumns`))
      (set `self.IsDestroyed` true)
      (`ActorComponent.K2_DestroyComponent` (`self.cobwebs_cobweb_001`))
      (bind _returnvalue (`GameplayStatics.GetActorOfClass` "/Game/Blueprints/BP_SpiderBoss.BP_SpiderBoss_C"))
      (`SceneComponent.K2_SetWorldLocation` (`Actor.RootComponent` _returnvalue) (- (`SceneComponent.K2_GetComponentLocation` (`self.DefaultSceneRoot`)) (* (`KismetMathLibrary.Vector_Up`) 100.0)) false false)
      (`GameplayStatics.PlaySound2D` "/Game/Sound/Music/SoundtrackAggressive.SoundtrackAggressive" 1.0 1.0 0.0 null null)
      (else
        (set `self.DestroyedColumns` 0)
        (for _array_element (`self.Columns`)
          (if (`/Game/Blueprints/BP_CobWebColumn.IsDestroyed` _array_element)
            (`/Engine/EditorBlueprintResources/StandardMacros.IncrementInt` (`self.DestroyedColumns`))))))))

(fn `UserConstructionScript`)