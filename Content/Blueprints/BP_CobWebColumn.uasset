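; BP_CobWebColumn is a destructible cobweb column that releases spiders when destroyed.
; Its ApplyDamage event subtracts from Health and shrinks the Scene component in two steps as health falls past two-thirds and one-third of MaxHealth.
; At zero health it destroys the mesh component, sets IsDestroyed to block further damage, and after a short delay spawns every class in SpidersToSpawn at the Scene's location.
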(event `/Game/Blueprints/BPI_Damageable.ApplyDamage`
  (params (Damage :type Integer))
  (if (not (`self.IsDestroyed`))
    (set `self.Health` (- (`self.Health`) Damage))
    (if (<= (`self.Health`) 0)
      (`ActorComponent.K2_DestroyComponent` (`self.StaticMesh`))
      (set `self.IsDestroyed` true)
      (`KismetSystemLibrary.Delay` 0.2)
      (for _array_element (`self.SpidersToSpawn`)
        (`|SpawnActorFromClass` _array_element (`KismetMathLibrary.MakeTransform` (`SceneComponent.K2_GetComponentLocation` (`self.Scene`))) "AdjustIfPossibleButAlwaysSpawn" "OverrideRootScale" null null))
      (elif (<= (`self.Health`) (/ (`self.MaxHealth`) 3))
        (`SceneComponent.SetWorldScale3D` (`self.Scene`) (0.3 0.3 0.3))
        (elif (<= (`KismetMathLibrary.Conv_IntToDouble` (`self.Health`)) (/ (`KismetMathLibrary.Conv_IntToDouble` (`self.MaxHealth`)) 1.5))
          (`SceneComponent.SetWorldScale3D` (`self.Scene`) (0.6 0.6 0.6)))))))

(fn `UserConstructionScript`)