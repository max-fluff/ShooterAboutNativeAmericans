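; BP_BossEnterTrigger is a one-shot trigger that starts the spider boss fight when the main character enters its box.
; At BeginPlay it hides the RockSet03D rock mesh by scaling it to zero.
; On the first overlap by BP_MainCharacter, it scales the rocks back up, likely blocking the way, and sets BP_SpiderBoss's BossStage to 1.
; A Triggered flag prevents repeat activation.
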(event `self.ReceiveBeginPlay`
  (`SceneComponent.SetWorldScale3D` (`self.RockSet03-D`) (0.0 0.0 0.0)))

(event `self.Box.OnComponentBeginOverlap`
  (params (OverlappedComponent :type "PrimitiveComponent Object Reference") (OtherActor :type "Actor Object Reference") (OtherComp :type "PrimitiveComponent Object Reference") (OtherBodyIndex :type Integer) (bFromSweep :type Boolean) (SweepResult :type "HitResult Structure (by ref)"))
  (cast `/Game/Blueprints/BP_MainCharacter` OtherActor)
  (if (not (`self.Triggered`))
    (set `self.Triggered` true)
    (`SceneComponent.SetRelativeScale3D` (`self.RockSet03-D`) (0.7 0.7 0.7))
    (bind _returnvalue (`GameplayStatics.GetActorOfClass` "/Game/Blueprints/BP_SpiderBoss.BP_SpiderBoss_C"))
    (set `/Game/Blueprints/BP_SpiderBoss.BossStage` 1 _returnvalue)))

(fn `UserConstructionScript`)