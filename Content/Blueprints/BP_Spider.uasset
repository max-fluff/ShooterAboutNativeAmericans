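; Spider enemy that wanders randomly while idle, chases the player on sight or noise, and bites at close range.
; An Idle/Alerted/Dead state drives AIMoveTo and controller focus, falling back to wandering when a chase move fails.
; Tick applies cooldown-limited bite damage and pauses the SpiderMove sound whenever the spider is stationary.
; Death disables collision, fully restores player stamina, and plays the death animation and screech.
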(event `self.ReceiveTick`
  (params (DeltaSeconds :type "Float (single-precision)"))
  (`|ExecutionSequence`
    (:`then_0`
      (set `self.TimeSinceLastAttack` (+ (`self.TimeSinceLastAttack`) DeltaSeconds))
      (if (`|EnumEquality` (`self.EnemyState`) "NewEnumerator1")
        (if (< (`KismetMathLibrary.VSize` (- (`SceneComponent.K2_GetComponentLocation` (`self.CapsuleComponent`)) (`SceneComponent.K2_GetComponentLocation` (`Character.Mesh` (`self.Player`))))) 150.0)
          (if (>= (`self.TimeSinceLastAttack`) (`self.AttackDelay`))
            (`/Game/Blueprints/BPI_Damageable.ApplyDamage` (`self.Player`) (`self.DamageAmount`))
            (`GameplayStatics.PlaySound2D` "/Game/Sound/Insects/Bite.Bite" 1.0 1.0 0.0 null null)
            (set `self.TimeSinceLastAttack` 0.0)))))
    (:`then_1`
      (`AudioComponent.SetPaused` (`self.SpiderMove`) (not (> (`KismetMathLibrary.VSize` (`MovementComponent.Velocity` (`self.CharacterMovement`))) 0.01))))))

(event `self.Init`
  (bind _spidermove (`self.SpiderMove`))
  (bind _asbp_main_character (cast `/Game/Blueprints/BP_MainCharacter` (`GameplayStatics.GetPlayerPawn` 0)))
  (set `self.Player` _asbp_main_character)
  (`KismetSystemLibrary.Delay` 0.2)
  (`self.StartIdling`)
  (`AudioComponent.Play` _spidermove 0.0)
  (`AudioComponent.SetPaused` _spidermove true))

(event `self.PawnSensing.OnHearNoise`
  (params (Instigator :type "Pawn Object Reference") (Location :type "Vector Structure (by ref)") (Volume :type "Float (single-precision)"))
  (if (`|EnumInequality` (`self.EnemyState`) "NewEnumerator2")
    (`self.StartFollowingPlayer` Instigator)))

(event `self.PawnSensing.OnSeePawn`
  (params (Pawn :type "Pawn Object Reference"))
  (`self.StartFollowingPlayer` Pawn))

(event `StartFollowingPlayer`
  (params (Actor :type "Actor Object Reference"))
  (if (`|EnumInequality` (`self.EnemyState`) "NewEnumerator2")
    (bind _asbp_main_character (cast `/Game/Blueprints/BP_MainCharacter` Actor))
    (`self.SetEnemyState` "NewEnumerator1")
    (`|AIMoveTo` self (0.0 0.0 0.0) _asbp_main_character 20.0
      (:`OnFail`
        (`self.SetEnemyState` "NewEnumerator0")))))

(event `StartIdling`
  (`|AIMoveTo` self (`NavigationSystemV1.K2_GetRandomReachablePointInRadius` (`CharacterMovementComponent.GetLastUpdateLocation` (`self.CharacterMovement`)) (* (`KismetMathLibrary.RandomFloat`) 1000.0) null null) null :!label _label
    (:`OnSuccess`
      _)
    (:`OnFail`
      _))
  (if (`|EnumEquality` (`self.EnemyState`) "NewEnumerator0")
    (`KismetSystemLibrary.Delay` (* (`KismetMathLibrary.RandomFloat`) 3.0))
    (if (`|EnumEquality` (`self.EnemyState`) "NewEnumerator0")
      (goto _label))))

(fn `OnDeath`
  (`SkeletalMeshComponent.PlayAnimation` (`self.Mesh`) "/Game/Models/Spider/Spider_Anim_Spider_Armature_die.Spider_Anim_Spider_Armature_die" false)
  (`GameplayStatics.PlaySoundAtLocation` "/Game/Sound/Insects/Screech.Screech" (`SceneComponent.K2_GetComponentLocation` (`self.CapsuleComponent`)) (struct) 1.0 1.0 0.0 null null null null))

(fn `OnStateBegin`
  (params (NewState :type "/Game/Enums/EEnemyState Enum" :default "NewEnumerator0"))
  (bind _returnvalue (`AIBlueprintHelperLibrary.GetAIController` self))
  (switch `/Game/Enums/EEnemyState` NewState
    (:`NewEnumerator0`
      (`self.StartIdling`)
      (`AIController.K2_SetFocus` _returnvalue null))
    (:`NewEnumerator1`
      (`AIController.K2_SetFocus` _returnvalue (`GameplayStatics.GetPlayerCharacter` 0)))
    (:`NewEnumerator2`
      (`AIController.K2_SetFocus` _returnvalue null)
      (`Controller.StopMovement` (`AIBlueprintHelperLibrary.GetAIController` self))
      (`PrimitiveComponent.SetCollisionEnabled` (`self.CapsuleComponent`) "NoCollision")
      (`PrimitiveComponent.SetCollisionEnabled` (`self.Mesh`) "NoCollision")
      (bind _asbp_main_character (cast `/Game/Blueprints/BP_MainCharacter` (`GameplayStatics.GetPlayerPawn` 0)))
      (`/Game/Blueprints/BP_MainCharacter.Event Restore Stamina` _asbp_main_character (`/Game/Blueprints/BP_MainCharacter.MaxStamina` _asbp_main_character))
      (`self.OnDeath`))))

(fn `UserConstructionScript`
  (`parent.UserConstructionScript`))