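; BP_Revolver is a six-round hitscan revolver weapon that starts with an empty cylinder.
; StartFire spends a round and line-traces forward from the actor on the Visibility channel, spawning a Niagara beam to the impact point only on a hit; no damage is applied here.
; Reload adds the given amount without clamping to MaxAmmo, and EndFire defers to the parent class.
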(fn `EndFire`
  (`parent.EndFire`))

(fn `Reload`
  (params (Amount :type Integer))
  (set `self.AmmoInWeapon` (+ (`self.AmmoInWeapon`) (`local.Amount`)))
  (return))

(fn `StartFire`
  (bind _returnvalue (`self.K2_GetActorLocation`))
  (if (> (`self.AmmoInWeapon`) 0)
    (`/Engine/EditorBlueprintResources/StandardMacros.DecrementInt` (`self.AmmoInWeapon`)
      (:`  `
        (bind (_outhit _returnvalue_2) (`KismetSystemLibrary.LineTraceSingle` _returnvalue (+ _returnvalue (* (`self.GetActorForwardVector`) (`self.HitLength`))) "TraceTypeQuery1"))
        (if _returnvalue_2
          (bind _returnvalue_3 (`NiagaraFunctionLibrary.SpawnSystemAtLocation` "/Game/Effects/N_Projectile.N_Projectile" (`self.K2_GetActorLocation`)))
          (`FXSystemComponent.SetVectorParameter` _returnvalue_3 "BeamEnd" (`.Location` (`GameplayStatics.BreakHitResult` _outhit))))))))

(fn `UserConstructionScript`
  (set `self.MaxAmmo` 6)
  (set `self.AmmoInWeapon` 0))