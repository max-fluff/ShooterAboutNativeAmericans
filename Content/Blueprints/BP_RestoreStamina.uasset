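; BP_RestoreStamina is a pickup that restores stamina to BP_MainCharacter.
; When the character overlaps its sphere while below max stamina, it calls EventRestoreStamina with the configured amount and plays a 2D sound.
; It then scales the scene root to zero and disables itself, reappearing after a short delay instead of being destroyed, so it can be collected repeatedly.
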(event `self.Sphere.OnComponentBeginOverlap`
  (params (OverlappedComponent :type "PrimitiveComponent Object Reference") (OtherActor :type "Actor Object Reference") (OtherComp :type "PrimitiveComponent Object Reference") (OtherBodyIndex :type Integer) (bFromSweep :type Boolean) (SweepResult :type "HitResult Structure (by ref)"))
  (if (`self.Enabled`)
    (bind _asbp_main_character (cast `/Game/Blueprints/BP_MainCharacter` OtherActor))
    (if (< (`/Game/Blueprints/BP_MainCharacter.StaminaLeft` _asbp_main_character) (`/Game/Blueprints/BP_MainCharacter.MaxStamina` _asbp_main_character))
      (`/Game/Blueprints/BP_MainCharacter.Event Restore Stamina` _asbp_main_character (`KismetMathLibrary.Conv_IntToDouble` (`self.StaminaRestoreAmount`)))
      (`SceneComponent.SetWorldScale3D` (`self.Scene`) (0.0 0.0 0.0))
      (set `self.Enabled` false)
      (`GameplayStatics.PlaySound2D` "/Game/Sound/Healing/Pipe.Pipe" 1.0 1.0 0.0 null null)
      (`KismetSystemLibrary.Delay` 5.0)
      (set `self.Enabled` true)
      (`SceneComponent.SetWorldScale3D` (`self.Scene`) (1.0 1.0 1.0)))))

(fn `UserConstructionScript`)