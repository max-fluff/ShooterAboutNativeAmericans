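; Helmeted spider enemy that wanders to random reachable points while idle and chases the player on sight.
; PawnSensing sends it toward noises or alerts it to follow BP_MainCharacter, returning to idle if that move fails.
; While alerted, its DamageCapsule damages overlapping BPI_Damageable actors other than walking enemies.
; OnStateBegin switches focus per EnemyState; death stops movement, disables collision, plays the death animation and refills player stamina.
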(event `self.Init`
  (`KismetSystemLibrary.Delay` 0.2)
  (`self.StartIdling`))

(event `self.PawnSensing.OnHearNoise`
  (params (Instigator :type "Pawn Object Reference") (Location :type "Vector Structure (by ref)") (Volume :type "Float (single-precision)"))
  (if (`|EnumInequality` (`self.EnemyState`) "NewEnumerator2")
    (`|AIMoveTo` null Location null 30.0)))

(event `self.PawnSensing.OnSeePawn`
  (params (Pawn :type "Pawn Object Reference"))
  (`self.StartFollowingPlayer` Pawn))

(event `StartFollowingPlayer`
  (params (Actor :type "Actor Object Reference"))
  (if (`|EnumInequality` (`self.EnemyState`) "NewEnumerator2")
    (bind _asbp_main_character (cast `/Game/Blueprints/BP_MainCharacter` Actor))
    (`self.SetEnemyState` "NewEnumerator1")
    (`|AIMoveTo` self (0.0 0.0 0.0) _asbp_main_character
      (:`OnFail`
        (`self.SetEnemyState` "NewEnumerator0")))))

(event `self.DamageCapsule.OnComponentBeginOverlap`
  (params (OverlappedComponent :type "PrimitiveComponent Object Reference") (OtherActor :type "Actor Object Reference") (OtherComp :type "PrimitiveComponent Object Reference") (OtherBodyIndex :type Integer) (bFromSweep :type Boolean) (SweepResult :type "HitResult Structure (by ref)"))
  (if (`|EnumEquality` (`self.EnemyState`) "NewEnumerator1")
    (cast `/Game/Blueprints/ABP_WalkingEnemy` OtherActor
      (:`CastFailed`
        (bind _asbpi_damageable (cast `/Game/Blueprints/BPI_Damageable` OtherActor))
        (`/Game/Blueprints/BPI_Damageable.ApplyDamage` _asbpi_damageable (`self.DamageAmount`))))))

(event `StartIdling`
  (`|AIMoveTo` self (`NavigationSystemV1.K2_GetRandomReachablePointInRadius` (`CharacterMovementComponent.GetLastUpdateLocation` (`self.CharacterMovement`)) (* (`KismetMathLibrary.RandomFloat`) 1000.0) null null) null :!label _label
    (:`OnSuccess`
      _)
    (:`OnFail`
      _))
  (if (`|EnumEquality` (`self.EnemyState`) "NewEnumerator0")
    (`KismetSystemLibrary.Delay` (* (`KismetMathLibrary.RandomFloat`) 3.0))
    (if (`|EnumEquality` (`self.EnemyState`) "NewEnumerator0")
      (goto _label))))

(fn `OnStateBegin`
  (params (NewState :type "/Game/Enums/EEnemyState Enum" :default "NewEnumerator0"))
  (bind _returnvalue (`AIBlueprintHelperLibrary.GetAIController` self))
  (switch `/Game/Enums/EEnemyState` NewState
    (:`NewEnumerator0`
      (`self.StartIdling`)
      (`AIController.K2_SetFocus` _returnvalue null))
    (:`NewEnumerator1`
      (`AIController.K2_SetFocus` _returnvalue (`GameplayStatics.GetPlayerCharacter` 0)))
    (:`NewEnumerator2`
      (`AIController.K2_SetFocus` _returnvalue null)
      (`Controller.StopMovement` (`AIBlueprintHelperLibrary.GetAIController` self))
      (`PrimitiveComponent.SetCollisionEnabled` (`self.CapsuleComponent`) "NoCollision")
      (`PrimitiveComponent.SetCollisionEnabled` (`self.Mesh`) "NoCollision")
      (`PrimitiveComponent.SetCollisionEnabled` (`self.skull_Skul_000`) "NoCollision")
      (bind _asbp_main_character (cast `/Game/Blueprints/BP_MainCharacter` (`GameplayStatics.GetPlayerPawn` 0)))
      (`/Game/Blueprints/BP_MainCharacter.Event Restore Stamina` _asbp_main_character (`/Game/Blueprints/BP_MainCharacter.MaxStamina` _asbp_main_character))
      (`SkeletalMeshComponent.PlayAnimation` (`self.Mesh`) "/Game/Models/Spider/Spider_Anim_Spider_Armature_die.Spider_Anim_Spider_Armature_die" false))))

(fn `UserConstructionScript`
  (`parent.UserConstructionScript`))