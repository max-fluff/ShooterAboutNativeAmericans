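; Exploding spider enemy that lights a ticking fuse near the player and detonates three seconds later.
; Overrides the parent's TryAttack and OnDeath, so death before ignition explodes it instantly, with an Ignited flag guarding against retriggering.
; Blow scans BPI_Damageable actors with capsules, applies linear distance-falloff damage within BlowRadius, damages itself and scales the dynamite to zero, with explosion effect and sound.
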(event `self.ReceiveBeginPlay`
  (`parent.ReceiveBeginPlay`)
  (`AudioComponent.Stop` (`self.Ticking`)))

(event `Blow`
  (bind _blowradius (`self.BlowRadius`))
  (`GameplayStatics.SpawnEmitterAtLocation` "/Game/StarterContent/Particles/P_Explosion.P_Explosion" (`SceneComponent.K2_GetComponentLocation` (`self.CapsuleComponent`)) (struct) (2.0 2.0 2.0))
  (`|ExecutionSequence`
    (:`then_0`
      (bind _outactors (`GameplayStatics.GetAllActorsWithInterface` "/Game/Blueprints/BPI_Damageable.BPI_Damageable_C"))
      (for _array_element _outactors
        (bind _returnvalue (`self.GetComponentByClass` _array_element "/Script/Engine.CapsuleComponent"))
        (`/Engine/EditorBlueprintResources/StandardMacros.IsValid` _returnvalue
          (:`Is Valid`
            (bind _asbpi_damageable (cast `/Game/Blueprints/BPI_Damageable` _array_element))
            (bind _returnvalue_2 (`KismetMathLibrary.VSize` (- (`SceneComponent.K2_GetComponentLocation` _returnvalue) (`SceneComponent.K2_GetComponentLocation` (`self.CapsuleComponent`)))))
            (if (< _returnvalue_2 _blowradius)
              (`self.ApplyDamage` _asbpi_damageable (`KismetMathLibrary.FTrunc` (* (- 1.0 (/ _returnvalue_2 _blowradius)) (`self.DamageAmount`)))))))))
    (:`then_1`
      (`GameplayStatics.PlaySoundAtLocation` "/Game/Sound/Blow/Blow.Blow" (`SceneComponent.K2_GetComponentLocation` (`self.CapsuleComponent`)) (struct) 1.0 1.0 0.0 null null null null)
      (`self.ApplyDamage` (`self.DamageAmount`))
      (`SceneComponent.SetWorldScale3D` (`self.Dynamite`) (0.0 0.0 0.0)))))

(event `Attack`
  (bind _ticking (`self.Ticking`))
  (if (not (`self.Ignited`))
    (set `self.Ignited` true)
    (`AudioComponent.Play` _ticking 0.0)
    (`KismetSystemLibrary.Delay` 3.0)
    (`AudioComponent.Stop` _ticking)
    (`self.Blow`)))

(fn `OnDeath`
  (if (not (`self.Ignited`))
    (set `self.Ignited` true)
    (`self.Blow`))
  (`parent.OnDeath`))

(fn `TryAttack`
  (params (DeltaTime :type "Float (double-precision)"))
  (if (< (`KismetMathLibrary.VSize` (- (`SceneComponent.K2_GetComponentLocation` (`self.CapsuleComponent`)) (`SceneComponent.K2_GetComponentLocation` (`Character.Mesh` (`self.Player`))))) 150.0)
    (`self.Attack`)))

(fn `UserConstructionScript`
  (`parent.UserConstructionScript`))