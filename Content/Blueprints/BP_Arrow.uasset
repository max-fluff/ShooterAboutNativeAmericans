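; Bow arrow projectile that damages what it hits, sticks in it and becomes an ammo pickup for BP_MainCharacter.
; A state machine (Unobtained, In Bow, In Air) switches collision and adds or removes a ProjectileMovement component, with launch speed from bow charge.
; Impact speed scales damage through BPI_Damageable and penetration depth before attaching.
; Tick returns an unobtained arrow to flight when its parent is invalid.
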(event `Fire`
  (params (BowCharge :type "Float (double-precision)") (Direction :type "Vector Structure"))
  (set `self.BowCharge` BowCharge)
  (set `self.Direction` Direction)
  (`self.SetArrowState` "NewEnumerator3"))

(event `self.ReceiveTick`
  (params (DeltaSeconds :type "Float (single-precision)"))
  (`/Engine/EditorBlueprintResources/StandardMacros.IsValid` (`self.Parent`)
    (:`Is Not Valid`
      (if (`|EnumEquality` (`self.ArrowState`) "NewEnumerator1")
        (`self.SetArrowState` "NewEnumerator3")))))

(event `self.Capsule.OnComponentBeginOverlap`
  (params (OverlappedComponent :type "PrimitiveComponent Object Reference") (OtherActor :type "Actor Object Reference") (OtherComp :type "PrimitiveComponent Object Reference") (OtherBodyIndex :type Integer) (bFromSweep :type Boolean) (SweepResult :type "HitResult Structure (by ref)")))

(event `self.StaticMesh.OnComponentBeginOverlap`
  (params (OverlappedComponent :type "PrimitiveComponent Object Reference") (OtherActor :type "Actor Object Reference") (OtherComp :type "PrimitiveComponent Object Reference") (OtherBodyIndex :type Integer) (bFromSweep :type Boolean) (SweepResult :type "HitResult Structure (by ref)"))
  (`self.HandleOverlap` OtherActor SweepResult OtherComp))

(fn `HandleOverlap`
  (params (OtherActor :type "Actor Object Reference") (HitResult :type "HitResult Structure") (OtherComp :type "PrimitiveComponent Object Reference"))
  (bind _otheractor (`local.OtherActor`))
  (bind (_min _max) (`StaticMeshComponent.GetLocalBounds` (`self.StaticMesh`)))
  (bind _returnvalue (- (.x _max) (.x _min)))
  (cast `/Game/Blueprints/BP_Arrow` OtherActor
    (:`CastFailed`
      (switch `/Game/Enums/EArrowState` (`self.ArrowState`)
        (:`NewEnumerator1`
          (bind _asbp_main_character (cast `/Game/Blueprints/BP_MainCharacter` _otheractor))
          (bind _added (`/Game/Blueprints/BP_MainCharacter.AddAmmo` _asbp_main_character 1 "NewEnumerator0"))
          (if _added
            (`GameplayStatics.PlaySound2D` "/Game/Sound/Healing/GrabAmmo.GrabAmmo" 1.0 1.0 0.0 null null)
            (`self.K2_DestroyActor`)))
        (:`NewEnumerator3`
          (cast `/Game/Blueprints/BP_MainCharacter` _otheractor
            (:`CastFailed`
              (`|ExecutionSequence`
                (:`then_0`
                  (bind _asbpi_damageable (cast `/Game/Blueprints/BPI_Damageable` (`local.OtherActor`)))
                  (`/Game/Blueprints/BPI_Damageable.ApplyDamage` _asbpi_damageable (`KismetMathLibrary.FTrunc` (* (`self.ArrowDamage`) (/ (`KismetMathLibrary.VSize` (`self.GetVelocity`)) 4000.0)))))
                (:`then_1`
                  (`self.SetArrowState` "NewEnumerator1")
                  (`self.K2_SetActorLocation` (- HitResult_ImpactPoint (* (`self.GetActorForwardVector`) (- _returnvalue (* (/ (`KismetMathLibrary.VSize` (`self.GetVelocity`)) 4000.0) (* _returnvalue (`self.MaxPenetrationPart`)))))))
                  (`self.K2_AttachToComponent` (`local.OtherComp`) "None" "KeepWorld" "KeepWorld" "KeepWorld")
                  (set `self.Parent` (`local.OtherActor`)))))))))))

(fn `OnStateBegin`
  (params (State :type "/Game/Enums/EArrowState Enum" :default "NewEnumerator0"))
  (bind _staticmesh (`self.StaticMesh`))
  (switch `/Game/Enums/EArrowState` State
    (:`NewEnumerator1`
      (`PrimitiveComponent.SetCollisionProfileName` _staticmesh "Projectile" true)
      (set `self.BowCharge` 0.0))
    (:`NewEnumerator2`
      (`PrimitiveComponent.SetCollisionProfileName` _staticmesh "NoCollision" true))
    (:`NewEnumerator3`
      (`PrimitiveComponent.SetCollisionProfileName` _staticmesh "Projectile" true)
      (bind _returnvalue (`AddComponent|NODE_AddProjectileMovementComponent-0`))
      (bind _output_get (set `self.ProjectileMovement` _returnvalue))
      (set `MovementComponent.Velocity` (* (`self.Direction`) (`KismetMathLibrary.Lerp` 100.0 4000.0 (`self.BowCharge`))) _output_get)
      (set `ProjectileMovementComponent.bRotationFollowsVelocity` true _output_get))))

(fn `OnStateEnd`
  (params (State :type "/Game/Enums/EArrowState Enum" :default "NewEnumerator0"))
  (bind _projectilemovement (`self.ProjectileMovement`))
  (switch `/Game/Enums/EArrowState` State
    (:`NewEnumerator1`
      (set `self.Parent` null))
    (:`NewEnumerator3`
      (`/Engine/EditorBlueprintResources/StandardMacros.IsValid` _projectilemovement
        (:`Is Valid`
          (`ActorComponent.K2_DestroyComponent` _projectilemovement))))))

(fn `SetArrowState`
  (params (NewState :type "/Game/Enums/EArrowState Enum" :default "NewEnumerator0"))
  (if (`|EnumInequality` NewState (`self.ArrowState`))
    (`self.OnStateEnd` (`self.ArrowState`))
    (bind _output_get (set `self.ArrowState` (`local.NewState`)))
    (`self.OnStateBegin` _output_get)))

(fn `UserConstructionScript`
  (`self.OnStateBegin` (`self.ArrowState`)))