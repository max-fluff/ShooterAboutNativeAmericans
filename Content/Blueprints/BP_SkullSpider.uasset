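; BP_SkullSpider is a spider character with a skull component, providing its movement feedback and death response.
; Tick calls the parent, then pauses the SkullMove component whenever movement velocity is near zero and resumes it when moving.
; OnDeath plays a non-looping death animation, disables the skull's collision, and plays screech and skull-crack sounds at the capsule's location.
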(event `self.ReceiveTick`
  (params (DeltaSeconds :type "Float (single-precision)"))
  (`parent.ReceiveTick` DeltaSeconds)
  (`AudioComponent.SetPaused` (`self.SkullMove`) (not (> (`KismetMathLibrary.VSize` (`MovementComponent.Velocity` (`self.CharacterMovement`))) 0.01))))

(fn `OnDeath`
  (bind _returnvalue (`SceneComponent.K2_GetComponentLocation` (`self.CapsuleComponent`)))
  (`SkeletalMeshComponent.PlayAnimation` (`self.Mesh`) "/Game/Models/Spider/Spider_Anim_Spider_Armature_die_2.Spider_Anim_Spider_Armature_die_2" false)
  (`PrimitiveComponent.SetCollisionEnabled` (`self.skull_Skul_000`) "NoCollision")
  (`GameplayStatics.PlaySoundAtLocation` "/Game/Sound/Insects/Screech.Screech" _returnvalue (struct) 1.0 1.0 0.0 null null null null)
  (`GameplayStatics.PlaySoundAtLocation` "/Game/Sound/Insects/SkullCrack.SkullCrack" _returnvalue (struct) 1.0 1.0 0.0 null null null null))

(fn `UserConstructionScript`
  (`parent.UserConstructionScript`))